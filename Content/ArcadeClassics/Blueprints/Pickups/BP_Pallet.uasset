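; BP_Pallet is a collectible pellet pickup that the player eats for points in an arcade classics game.
; An overlap on its mesh counts only when it comes from the player's Eatcollision component.
; The pellet then plays an eat sound, destroys itself and notifies the gameplay GameMode to decrease the pellet count.
; It also adds its points to the GameInstance score and runs the 1-up check.
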(event `self.SM_Pallet.OnComponentBeginOverlap`
  (params (OverlappedComponent :type "PrimitiveComponent Object Reference") (OtherActor :type "Actor Object Reference") (OtherComp :type "PrimitiveComponent Object Reference") (OtherBodyIndex :type Integer) (bFromSweep :type Boolean) (SweepResult :type "HitResult Structure (by ref)"))
  (bind _asbp_player (cast `/Game/ArcadeClassics/Blueprints/Characters/BP_Player` OtherActor))
  (if (== OtherComp (`/Game/ArcadeClassics/Blueprints/Characters/BP_Player.Eatcollision` _asbp_player))
    (`|ExecutionSequence`
      (:`then_0`
        ;[1 1 1] Pallet eaten handling
        (`GameplayStatics.SpawnSound2D` "/Game/ArcadeClassics/Audio/SFX_Eat_Cue.SFX_Eat_Cue" 1.0 1.0 0.0 null)
        (`self.K2_DestroyActor`))
      (:`then_1`
        ;[1 1 1] Decrease Pallet Count
        (bind _asbp_game_mode_gameplay (cast `/Game/ArcadeClassics/Blueprints/Framework/BP_GameMode_Gameplay` (`GameplayStatics.GetGameMode`)))
        (`/Game/ArcadeClassics/Blueprints/Framework/BP_GameMode_Gameplay.AtePellet` _asbp_game_mode_gameplay))
      (:`then_2`
        ;[1 1 1] Increment Score
        (bind _asbp_game_instance (cast `/Game/ArcadeClassics/Blueprints/Framework/BP_GameInstance` (`GameplayStatics.GetGameInstance`)))
        (`/Game/ArcadeClassics/Blueprints/Framework/BP_GameInstance.AddPoints` _asbp_game_instance (`self.PalletPoints`))
        (`/Game/ArcadeClassics/Blueprints/Framework/BP_GameInstance.1upCheck` _asbp_game_instance)))))

(fn `UserConstructionScript`)