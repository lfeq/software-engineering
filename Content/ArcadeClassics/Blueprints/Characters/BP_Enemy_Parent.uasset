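; Parent Blueprint for arcade maze-style enemies that kill the player on overlap, or get eaten while vulnerable.
; PowerPelletEaten starts a timeline that switches visual states through two vulnerable phases, then restores regular.
; Eaten enemies hide, teleport to EnemyRespawnLocation and reappear after delays; killing the player resets all enemies through the same path.
; Dispatcher calls signal vulnerability and player death; the node storing the respawn location is unconnected here.
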(event `Reset Enemies at Home`
  ;[1 1 1] Enemy  reset to house
  (`self.EnemySpawnFX`)
  ;[1 1 1] Enemy eaten respawn backhome
  (`self.K2_SetActorLocation` (`self.EnemyRespawnLocation`) :!label _label)
  (`KismetSystemLibrary.Delay` 2.0)
  (`GameplayStatics.SpawnEmitterAtLocation` "/Game/InfinityBladeEffects/Effects/FX_Monsters/FX_Monster_Deaths/P_Monster_Death_Large.P_Monster_Death_Large" (`self.EnemyRespawnLocation`))
  (`PrimitiveComponent.SetCollisionResponseToChannel` (`self.Player_Collision`) "ECC_Pawn" "ECR_Overlap")
  (`KismetSystemLibrary.Delay` 1.0)
  (`self.SetActorHiddenInGame` false))

(event `self.Player_Collision.OnComponentBeginOverlap`
  (params (OverlappedComponent :type "PrimitiveComponent Object Reference") (OtherActor :type "Actor Object Reference") (OtherComp :type "PrimitiveComponent Object Reference") (OtherBodyIndex :type Integer) (bFromSweep :type Boolean) (SweepResult :type "HitResult Structure (by ref)"))
  ;[1 1 1] Enemy touched player
  (bind _asbp_player (cast `/Game/ArcadeClassics/Blueprints/Characters/BP_Player` OtherActor))
  (`/Engine/EditorBlueprintResources/StandardMacros.IsValid` _asbp_player
    (:`Is Valid`
      (if (`self.bIsVulnerable?`)
        ;[1 1 1] Enemy eaten respawn backhome
        (`self.EnemyEatenFX`)
        (`PrimitiveComponent.SetCollisionResponseToChannel` (`self.Player_Collision`) "ECC_Pawn" "ECR_Ignore")
        (set `self.bIsVulnerable?` false)
        (`self.EnemyStateRegular`)
        (goto _label)
        (else
          ;[1 1 1] Send all enemies home
          (`self.KilledPlayer`)
          (`KismetSystemLibrary.Delay` 2.5)
          (`self.Reset Enemies at Home` (`self.Enemies`)))))))

(event `self.ReceiveBeginPlay`
  (`|ExecutionSequence`
    (:`then_0`
      ;[1 1 1] Reference to all enemies
      (bind _outactors (`GameplayStatics.GetAllActorsOfClass` "BP_Enemy_Parent_C"))
      (set `self.Enemies` _outactors))))

(event `PowerPelletEaten`
  ;[1 1 1] Manage vulnerable state
  (set `self.bIsVulnerable?` true)
  (`self.Vulnerable`)
  (`Timeline|VulnerabilitySequence` :!via `PlayFromStart`
    (:`Finished`
      (`self.EnemyStateRegular`)
      (set `self.bIsVulnerable?` false)
      (`self.NotVulnerable`))
    (:`StartPhase01`
      (`self.EnemyStateVulnerable01`))
    (:`StartPhase02`
      (if (`self.bIsVulnerable?`)
        (`self.EnemyStateVulnerable02`)))))

(fn `EnemyEatenFX`
  (`GameplayStatics.SpawnEmitterAtLocation` "/Game/ArcadeClassics/Particles/P_Death.P_Death" (`SceneComponent.K2_GetComponentLocation` (`self.CapsuleComponent`)))
  (`GameplayStatics.PlaySound2D` "/Game/ArcadeClassics/Audio/SFX_EatEnemy_Cue.SFX_EatEnemy_Cue" 1.0 1.0 0.0 null null)
  (`self.SetActorHiddenInGame` true))

(fn `EnemySpawnFX`
  (`GameplayStatics.SpawnEmitterAtLocation` "/Game/ArcadeClassics/Particles/P_SpawnEnemy.P_SpawnEnemy" (`SceneComponent.K2_GetComponentLocation` (`self.CapsuleComponent`)))
  (`self.SetActorHiddenInGame` true))

(fn `EnemyStateRegular`
  (`SceneComponent.SetVisibility` (`self.Enemy_Vulnerable_01`) false false)
  (`SceneComponent.SetVisibility` (`self.Enemy_Vulnerable_02`) false false)
  (`SceneComponent.SetVisibility` (`self.Enemy_Down`) true false))

(fn `EnemyStateVulnerable01`
  (`SceneComponent.SetVisibility` (`self.Enemy_Vulnerable_02`) false false)
  (`SceneComponent.SetVisibility` (`self.Enemy_Down`) false false)
  (`SceneComponent.SetVisibility` (`self.Enemy_Vulnerable_01`) true false))

(fn `EnemyStateVulnerable02`
  (`SceneComponent.SetVisibility` (`self.Enemy_Vulnerable_01`) false false)
  (`SceneComponent.SetVisibility` (`self.Enemy_Down`) false false)
  (`SceneComponent.SetVisibility` (`self.Enemy_Vulnerable_02`) true false))

(fn `UserConstructionScript`)