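; Gameplay game mode for a Pac-Man-style level, running intro, lives, pellet progress and end screens.
; BeginPlay creates the HUD, blends cameras before enabling input, counts pellets and schedules one random fruit or speed power-up spawn.
; Enemy kill events deduct lives and can trigger game over, while kill and vulnerability events also drive music.
; AtePellet decrements the total, then at zero stops the player, closes enemy gates and shows the level-complete menu.
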(event `ListenForKilledPlayer`
  ;[1 1 1] Listen to Killed Player
  (add `/Game/ArcadeClassics/Blueprints/Characters/BP_Enemy_Parent.KilledPlayer` (`self.Enemies`) (delegate `KilledPlayer_Event_1`)))

(event `KilledPlayer_Event_1`
  ;[1 1 1] Listen to Killed Player
  (`|ExecutionSequence`
    (:`then_0`
      ;[1 1 1] Subtract live
      (`KismetSystemLibrary.Delay` 1.75)
      (bind _updatedlives (`/Game/ArcadeClassics/Blueprints/Framework/BP_GameInstance.SubtractLives` (`self.GameInstance`) 1))
      (if (<= _updatedlives 0)
        ;[1 1 1] Game over menu
        (`KismetSystemLibrary.Delay` 1.5)
        (bind _returnvalue (`|CreateWidget` "/Game/ArcadeClassics/UMG/GameOverMenu.GameOverMenu_C"))
        (bind _output_get (set `self.GameOver` _returnvalue))
        (`UserWidget.AddToViewport` _output_get 0)
        (`GameplayStatics.SetGamePaused` true)))
    (:`then_1`
      ;[1 1 1] Play Life Lost Animation
      (`/Game/ArcadeClassics/UMG/HUD.LifeLost` (`self.HUD`)))))

(event `self.ReceiveBeginPlay`
  (bind _returnvalue (`GameplayStatics.GetPlayerCharacter` 0))
  (bind _array (`|MakeArray` (`self.GoodieSpawn_01`) (`self.GoodieSpawn_02`)))
  (`|ExecutionSequence`
    (:`then_2`
      ;[1 1 1] Create Reference To HUD
      (bind _returnvalue_2 (`|CreateWidget` "/Game/ArcadeClassics/UMG/HUD.HUD_C"))
      (bind _output_get (set `self.HUD` _returnvalue_2))
      (`UserWidget.AddToViewport` _output_get 0)
      (bind _returnvalue_3 (`|CreateWidget` "/Game/ArcadeClassics/UMG/GameStartNotify.GameStartNotify_C"))
      (`KismetSystemLibrary.Delay` 5.0)
      (`UserWidget.AddToViewport` _returnvalue_3 0))
    (:`then_3`
      ;[1 1 1] Set Reference to Game Instance
      (bind _asbp_game_instance (cast `/Game/ArcadeClassics/Blueprints/Framework/BP_GameInstance` (`GameplayStatics.GetGameInstance`)))
      (set `self.GameInstance` _asbp_game_instance)
      ;[1 1 1] Set Reference to Player
      (bind _asbp_player (cast `/Game/ArcadeClassics/Blueprints/Characters/BP_Player` (`GameplayStatics.GetPlayerCharacter` 0)))
      (set `self.PlayerRef` _asbp_player)
      ;[1 1 1] Reference to all enemies
      (bind _outactors (`GameplayStatics.GetAllActorsOfClass` "/Game/ArcadeClassics/Blueprints/Characters/BP_Enemy_Parent.BP_Enemy_Parent_C"))
      (set `self.Enemies` _outactors)
      ;[1 1 1] Initialices Listening of player killed event
      (`self.ListenForKilledPlayer`))
    (:`then_4`
      ;[1 1 1] Total Pellets existing in level
      (bind _outactors_2 (`GameplayStatics.GetAllActorsOfClass` "/Game/ArcadeClassics/Blueprints/Pickups/BP_Pallet.BP_Pallet_C"))
      (bind _output_get_2 (set `self.TotalRegularPellets` (`KismetArrayLibrary.Array_Length` _outactors_2))))
    (:`then_5`
      (bind _outactors_3 (`GameplayStatics.GetAllActorsOfClass` "/Game/ArcadeClassics/Blueprints/Pickups/BP_PowerPallet.BP_PowerPallet_C"))
      (bind _output_get_3 (set `self.TotalPowerPellets` (`KismetArrayLibrary.Array_Length` _outactors_3)))
      (set `self.TotalPellets` (+ _output_get_2 _output_get_3)))
    (:`then_6`
      ;[1 1 1] Intro camera aimation
      (bind _returnvalue_4 (`|SpawnActorFromClass` "/Script/Engine.CameraActor" (`KismetMathLibrary.MakeTransform` (`self.CamIntro01_Loc`) (`self.CamIntro01_Rot`)) "Undefined" "OverrideRootScale" null null))
      (`PlayerController.SetViewTargetWithBlend` (`GameplayStatics.GetPlayerController` 0) _returnvalue_4 0.0 "VTBlend_Linear" 0.0 false)
      ;[1 0.8546 0.165] Gameplay Camera
      (`self.DisableInput` (`GameplayStatics.GetPlayerCharacter` 0) (`GameplayStatics.GetPlayerController` 0))
      (bind _returnvalue_5 (`|SpawnActorFromClass` "/Script/Engine.CameraActor" (`KismetMathLibrary.MakeTransform` (`self.CamGameplay_Loc`) (`self.CamGameplay_Rot`)) "Undefined" "OverrideRootScale" null null))
      (`PlayerController.SetViewTargetWithBlend` (`GameplayStatics.GetPlayerController` 0) _returnvalue_5 6.8 "VTBlend_Linear" 0.0 false)
      (`KismetSystemLibrary.Delay` 7.0)
      (`self.EnableInput` _returnvalue (`GameplayStatics.GetPlayerController` 0))
      (bind _asbp_player_2 (cast `/Game/ArcadeClassics/Blueprints/Characters/BP_Player` _returnvalue))
      (set `/Game/ArcadeClassics/Blueprints/Characters/BP_Player.bAllowedToMove?` true _asbp_player_2))
    (:`then_7`
      ;[1 1 1] Fruit/powerup spawn
      (`KismetSystemLibrary.Delay` (`KismetMathLibrary.RandomFloatInRange` 25.0 50.0))
      (if (`self.bGoodieSpawnOk?`)
        (bind _output_get_4 (set `self.GoodieSpawnLocals` _array))
        (switch `int` (`KismetMathLibrary.RandomIntegerInRange` 0 2)
          (:`0`
            (bind _returnvalue_6 (`KismetMathLibrary.Conv_VectorToTransform` (`|GetArrayItem` _output_get_4 (`KismetMathLibrary.RandomIntegerInRange` 0 (- (`KismetArrayLibrary.Array_Length` _array) 1)))))
            (`|SpawnActorFromClass` "/Game/ArcadeClassics/Blueprints/Pickups/BP_Food_Cherry.BP_Food_Cherry_C" _returnvalue_6 "Undefined" "OverrideRootScale" null null))
          (:`1`
            (`|SpawnActorFromClass` "/Game/ArcadeClassics/Blueprints/Pickups/BP_Food_Orange.BP_Food_Orange_C" _returnvalue_6 "Undefined" "OverrideRootScale" null null))
          (:`2`
            (`|SpawnActorFromClass` "/Game/ArcadeClassics/Blueprints/Pickups/BP_PowerUpSPeed.BP_PowerUpSPeed_C" _returnvalue_6 "Undefined" "OverrideRootScale" null null)))))
    (:`then_8`
      (`|ExecutionSequence`
        (:`then_0`
          ;[1 1 1] Music stops / resumes after player dies
          (add `/Game/ArcadeClassics/Blueprints/Characters/BP_Enemy_Parent.KilledPlayer` (`self.Enemies`) (delegate `KilledPlayer_Event_0`)))
        (:`then_1`
          ;[1 1 1] Vuulnerable or not
          (add `/Game/ArcadeClassics/Blueprints/Characters/BP_Enemy_Parent.Vulnerable` (`self.Enemies`) (delegate `Vulnerable_Event_0`)))
        (:`then_2`
          (add `/Game/ArcadeClassics/Blueprints/Characters/BP_Enemy_Parent.NotVulnerable` (`self.Enemies`) (delegate `NotVulnerable_Event_0`))
          (`AudioComponent.SetPaused` (`self.Music_Gameplay`) false)
          (`AudioComponent.Stop` (`self.Music_Vulnerable`)))
        (:`then_3`
          ;[1 1 1] Level complete (Stop music)
          (add `self.LevelCompleted` (delegate `LevelCompleted_Event`)))))))

(event `AtePellet`
  (bind _playerref (`self.PlayerRef`))
  ;[1 1 1] Level complete
  (bind _result (`/Engine/EditorBlueprintResources/StandardMacros.DecrementInt` (`self.TotalPellets`))
    (:`  `
      (bind _output_get (set `self.TotalPellets` _result))
      (if (<= _output_get 0)
        (set `self.bGoodieSpawnOk?` false)
        (`|ExecutionSequence`
          (:`then_0`
            (`self.DisableInput` (`GameplayStatics.GetPlayerCharacter` 0) (`GameplayStatics.GetPlayerController` 0))
            (set `CharacterMovementComponent.MaxWalkSpeed` 0.0 (`Character.CharacterMovement` _playerref))
            (set `/Game/ArcadeClassics/Blueprints/Characters/BP_Player.bShouldPlayerGobble` false _playerref))
          (:`then_1`
            ;[1 1 1] Level complete menu
            (`self.LevelCompleted`)
            (`KismetSystemLibrary.Delay` 2.0)
            (bind _returnvalue (`|CreateWidget` "/Game/ArcadeClassics/UMG/LevelCompleteMenu.LevelCompleteMenu_C"))
            (bind _output_get_2 (set `self.LevelComplete` _returnvalue))
            (`UserWidget.AddToViewport` _output_get_2 0)
            (`GameplayStatics.SetGamePaused` true))
          (:`then_2`
            (for _array_element (`self.Enemies`)
              (`/Game/ArcadeClassics/Blueprints/Characters/BP_Enemy_Parent.CloseEnemyNavGate` _array_element))))))))

(event `KilledPlayer_Event_0`
  (bind _music_gameplay (`self.Music_Gameplay`))
  ;[1 1 1] Music stops / resumes after player dies
  (`|ExecutionSequence`
    (:`then_0`
      (`AudioComponent.Stop` _music_gameplay))
    (:`then_1`
      (`KismetSystemLibrary.Delay` 7.0)
      (`AudioComponent.FadeIn` _music_gameplay 0.5 1.0 7.0 "Linear"))))

(event `Vulnerable_Event_0`
  (bind _music_vulnerable (`self.Music_Vulnerable`))
  ;[1 1 1] Vuulnerable or not
  (`AudioComponent.SetPaused` (`self.Music_Gameplay`) true)
  (if (not (`AudioComponent.IsPlaying` _music_vulnerable))
    (`AudioComponent.Play` _music_vulnerable 0.0)))

(event `NotVulnerable_Event_0`
  ;[1 1 1] Vuulnerable or not
)

(event `LevelCompleted_Event`
  ;[1 1 1] Level complete (Stop music)
  (`KismetSystemLibrary.Delay` 0.1)
  (`AudioComponent.Stop` (`self.Music_Gameplay`))
  (`AudioComponent.Stop` (`self.Music_Vulnerable`)))

(fn `UserConstructionScript`)